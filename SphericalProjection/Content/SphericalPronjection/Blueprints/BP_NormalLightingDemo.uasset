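; BP_NormalLightingDemo is a demo Blueprint that feeds a light direction to the materials on its skeletal mesh.
; Its Construction Script creates a dynamic material instance for each material slot when LightDirectionSource is valid, storing them in an array.
; Each instance's LightDirection vector parameter receives that actor's forward vector at construction time.
; The Reflesh flag resets on every construction, apparently serving as an editor refresh toggle.
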(fn ConstructionScript
  (Variables|Default|SetReflesh false)
  (Utilities|IsValid (Variables|Default|GetLightDirectionSource)
    (:Is%20Valid
      (Utilities|Array|Clear (Variables|Default|GetDynamicMaterialInstances))
      (for (_ _array_index) (Rendering|Material|GetMaterials (Variables|Default|GetSkeletalMesh))
        (bind _returnvalue (Rendering|Material|CreateDynamicMaterialInstance (Variables|Default|GetSkeletalMesh) _array_index 0 :!class /Script/Engine.PrimitiveComponent))
        (Utilities|Array|Add (Variables|Default|GetDynamicMaterialInstances) _returnvalue)
        (Rendering|Material|SetVectorParameterValue _returnvalue "LightDirection" (Math|Conversions|ToLinearColor(Vector) (Math|Vector|GetForwardVector (Transformation|GetActorRotation (Variables|Default|GetLightDirectionSource)))) :!class /Script/Engine.MaterialInstanceDynamic)))))