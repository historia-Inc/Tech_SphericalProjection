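; BP_PlayerPawn is a player pawn that maps input axes to free movement and look control.
; Forward and right inputs move along the control rotation's axes, so forward follows camera pitch, while MoveUp always moves along world up.
; Turn and LookUp feed controller yaw and pitch directly, with no scaling, and the construction script is empty.
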(event Input|AxisEvents|InputAxisTurn
  (params (AxisValue :type Float%20%28single-precision%29))
  (Pawn|Input|AddControllerYawInput AxisValue))

(event Input|AxisEvents|InputAxisLookUp
  (params (AxisValue :type Float%20%28single-precision%29))
  (Pawn|Input|AddControllerPitchInput AxisValue))

(event Input|AxisEvents|InputAxisMoveUp
  (params (AxisValue :type Float%20%28single-precision%29))
  (Pawn|Input|AddMovementInput (Math|Vector|GetUpVector "0, 0, 0") AxisValue false))

(event Input|AxisEvents|InputAxisMoveForward
  (params (AxisValue :type Float%20%28single-precision%29))
  (Pawn|Input|AddMovementInput (.X (Math|Rotator|GetAxes (Pawn|GetControlRotation :!class /Script/Engine.Pawn))) AxisValue false))

(event Input|AxisEvents|InputAxisMoveRight
  (params (AxisValue :type Float%20%28single-precision%29))
  (Pawn|Input|AddMovementInput (.Y (Math|Rotator|GetAxes (Pawn|GetControlRotation :!class /Script/Engine.Pawn))) AxisValue false))

(fn ConstructionScript)